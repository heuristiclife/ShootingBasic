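; BP_EnemyGOD is an enemy spawner actor that periodically creates BP_Enemy instances at its own transform.
; Tick accumulates elapsed time and, once it reaches CreateTime, calls CreateEnemy and resets the timer to zero.
; CreateEnemy spawns the enemy with collision handling set to always spawn, so overlaps never block it.
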(event EventBeginPlay)

(event Collision|EventActorBeginOverlap
  (params (OtherActor :type Actor%20Object%20Reference)))

(event EventTick
  (params (DeltaSeconds :type Float%20%28single-precision%29))
  ;[1 1 1] 시간이 흘러야 한다
  (bind _output_get (Variables|Default|SetCurrentTime (+ DeltaSeconds (Variables|Default|GetCurrentTime))))
  ;[1 1 1] 생성시간 체크
  (if (>= _output_get (Variables|Default|GetCreateTime))
    ;[1 1 1] 적을 생성한다
    (CallFunction|CreateEnemy)
    ;[1 1 1] 경과시간 초기화
    (Variables|Default|SetCurrentTime 0.0)))

(fn ConstructionScript)

(fn CreateEnemy
  (Game|SpawnActorfromClass "/Game/Blueprints/BP_Enemy.BP_Enemy_C" (Transformation|GetActorTransform) "AlwaysSpawn" 0 0))