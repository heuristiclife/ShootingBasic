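; BP_Enemy is an enemy actor that flies in a straight line and destroys itself along with what it hits.
; On BeginPlay it finds BP_Player and picks a fixed direction: toward the player half the time, otherwise straight down, also the fallback without a valid target.
; Tick moves it with sweep.
; Any Box overlap plays a sound and explosion, but both actors are destroyed only if the other is not a BP_Enemy.
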(event OnComponentBeginOverlap(StaticMesh)
  (params (OverlappedComponent :type Primitive%20Component%20Object%20Reference) (OtherActor :type Actor%20Object%20Reference) (OtherComp :type Primitive%20Component%20Object%20Reference) (OtherBodyIndex :type Integer) (bFromSweep :type Boolean) (SweepResult :type Hit%20Result%20Structure%20%28by%20ref%29))
  ;[1 1 1] 충돌했을 때 너도 죽고 나도 죽는다(Component 별 처리, static mesh 기준)
)

(event OnComponentBeginOverlap(Box)
  (params (OverlappedComponent :type Primitive%20Component%20Object%20Reference) (OtherActor :type Actor%20Object%20Reference) (OtherComp :type Primitive%20Component%20Object%20Reference) (OtherBodyIndex :type Integer) (bFromSweep :type Boolean) (SweepResult :type Hit%20Result%20Structure%20%28by%20ref%29))
  (Audio|PlaySound2D 0 1.0 1.0 0.0 0 0)
  (Effects|SpawnEmitteratLocation "/Game/StarterContent/Particles/P_Explosion.P_Explosion" (Transformation|GetActorLocation) "0, 0, 0" "2.000000,2.000000,2.000000")
  (Utilities|Casting|CastToBP_Enemy OtherActor
    (:CastFailed
      ;[1 1 1] 충돌했을 때 너도 죽고 나도 죽는다(Actor)
      (Actor|DestroyActor OtherActor)
      (Actor|DestroyActor))))

(event EventTick
  (params (DeltaSeconds :type Float%20%28single-precision%29))
  (Transformation|SetActorLocation (+ (Transformation|GetActorLocation) (* (* (Variables|Default|GetDirection) (Variables|Default|GetSpeed)) DeltaSeconds)) true false))

(event EventBeginPlay
  ;[1 1 1] 타겟을 찾는다
  (bind _returnvalue (Actor|GetActorOfClass "/Game/Blueprints/BP_Player.BP_Player_C"))
  (Variables|Default|SetTarget _returnvalue)
  ;[1 1 1] 방향을 찾는다
  (CallFunction|FindDirection))

(event Collision|EventActorBeginOverlap
  (params (OtherActor :type Actor%20Object%20Reference))
  ;[1 1 1] 충돌했을 때 너도 죽고 나도 죽는다(Actor)
)

(fn ConstructionScript)

(fn FindDirection
  (bind _target (Variables|Default|GetTarget))
  (Utilities|IsValid _target
    (:Is%20Valid
      (if (<= (Math|Random|RandomIntegerinRange 1 100) 50)
        (Variables|Default|SetDirection (Math|Vector|Normalize (- (Transformation|GetActorLocation _target) (Transformation|GetActorLocation))))
        (else
          (Variables|Default|SetDirection "0, 0,-1.000000" :!label _label))))
    (:Is%20Not%20Valid
      (goto _label))))