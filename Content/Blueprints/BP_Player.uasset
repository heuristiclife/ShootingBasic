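; BP_Player is the player-controlled actor that moves in the YZ plane and fires bullets.
; Horizontal and Vertical axis inputs share one Direction setter, and Tick moves the actor along the normalized Direction by Speed and delta time with sweep.
; The fire press calls CreateBullet, which spawns BP_Bullet at the actor's transform and plays a 2D shot sound.
; A preloaded AudioBullet playback call is left unconnected.
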(event EventBeginPlay
  (Input|EnableInput (Game|GetPlayerController 0)))

(event Collision|EventActorBeginOverlap
  (params (OtherActor :type Actor%20Object%20Reference)))

(event EventTick
  (params (DeltaSeconds :type Float%20%28single-precision%29))
  ;[1 1 1] P
  (Transformation|SetActorLocation (+ (* (* (Math|Vector|Normalize (Variables|Default|GetDirection)) (Variables|Default|GetSpeed)) DeltaSeconds) (Transformation|GetActorLocation)) true false))

(event Input|ActionEvents|InputActionfire
  (params (Key :type Key%20Structure :default "None"))
  ;[1 1 1] 발사버튼을 누르면 총알 발사
  (:Pressed
    (CallFunction|CreateBullet)))

(event Input|AxisEvents|InputAxisVertical
  (params (AxisValue :type Float%20%28single-precision%29))
  (Variables|Default|SetDirection (Math|Vector|MakeVector 0.0 (stale Input|AxisEvents|InputAxisHorizontal AxisValue) AxisValue)))

(event Input|AxisEvents|InputAxisHorizontal
  (params (AxisValue :type Float%20%28single-precision%29))
  (Variables|Default|SetDirection (Math|Vector|MakeVector 0.0 AxisValue (stale Input|AxisEvents|InputAxisVertical AxisValue))))

(fn ConstructionScript)

(fn CreateBullet
  (Game|SpawnActorfromClass "/Game/Blueprints/BP_Bullet.BP_Bullet_C" (Transformation|GetActorTransform) "AlwaysSpawn" 0 0)
  ;[1 1 1] 쏠 때마다 생성
  (Audio|PlaySound2D "/Game/Sounds/Audio_Bullet.Audio_Bullet" 1.0 1.0 0.0 0 0))